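; Platform_BP is a moving platform that shuttles its Cube back and forth between two points.
; The construction script places StartPosition and EndPosition markers at the PositionStartLoc and PositionEndLoc variables.
; On BeginPlay, latent MoveComponentTo calls move the Cube to the start marker, then to the end marker over TravelTime, looping endlessly.
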(event `self.ReceiveBeginPlay`
  (`KismetSystemLibrary.MoveComponentTo` (`self.Cube`) (`SceneComponent.RelativeLocation` (`self.StartPosition`)) (struct) false false (`self.TravelTime`) :!label _label)
  (`KismetSystemLibrary.MoveComponentTo` (`self.Cube`) (`SceneComponent.RelativeLocation` (`self.EndPosition`)) (struct) false false (`self.TravelTime`))
  (goto _label))

(fn `UserConstructionScript`
  (`SceneComponent.K2_SetRelativeLocation` (`self.StartPosition`) (`self.PositionStartLoc`) false false)
  (`SceneComponent.K2_SetRelativeLocation` (`self.EndPosition`) (`self.PositionEndLoc`) false false))