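; Side-scroller hazard enemy that shuttles between two points and kills the player character on contact with its spinning blades.
; BeginPlay loops MoveComponentTo on the cube between the start and end markers over a set travel time, while Tick rotates the blades.
; The construction script places both markers from configurable locations, and blade collision overlap calls Death on the side-scroller character.
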(event `self.ReceiveBeginPlay`
  (`KismetSystemLibrary.MoveComponentTo` (`self.Cube`) (`SceneComponent.RelativeLocation` (`self.StartPosition`)) (struct) false false (`self.TravelTime`) :!label _label)
  (`KismetSystemLibrary.MoveComponentTo` (`self.Cube`) (`SceneComponent.RelativeLocation` (`self.EndPosition`)) (struct) false false (`self.TravelTime`))
  (goto _label))

(event `self.ReceiveTick`
  (params (DeltaSeconds :type "Float (single-precision)"))
  (`SceneComponent.K2_AddWorldRotation` (`self.Blades`) (struct :`Yaw` 10.0) false false))

(event `self.BladeCollusion.OnComponentBeginOverlap`
  (params (OverlappedComponent :type "PrimitiveComponent Object Reference") (OtherActor :type "Actor Object Reference") (OtherComp :type "PrimitiveComponent Object Reference") (OtherBodyIndex :type Integer) (bFromSweep :type Boolean) (SweepResult :type "HitResult Structure (by ref)"))
  (bind _asside_scroller_character (cast `/Game/SideScrollerBP/Blueprints/SideScrollerCharacter` OtherActor))
  (`/Game/SideScrollerBP/Blueprints/SideScrollerCharacter.Death` _asside_scroller_character))

(fn `UserConstructionScript`
  (`SceneComponent.K2_SetRelativeLocation` (`self.StartPosition`) (`self.PositionStartLoc`) false false)
  (`SceneComponent.K2_SetRelativeLocation` (`self.EndPosition`) (`self.PositionEndLoc`) false false))